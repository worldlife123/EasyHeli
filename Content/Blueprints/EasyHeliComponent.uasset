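; Helper component for BP_Generic_Helicopter that adds hover assist and blade collision warnings.
; DoHovering, not called within this component, turns yaw-relative velocity into smoothed, capped pitch and roll corrections for the movement component's rotation input.
; A looping timer box-traces main and tail blade bounds along predicted velocity while the engine runs, updating WarningOn only on change.
; Debug trace drawing and rotation printing remain enabled.
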(event `self.ReceiveBeginPlay`
  (bind _asbp_generic_helicopter (cast `/Game/Vehicles/UH60M/BP_Generic_Helicopter` (`self.GetOwner`)))
  (set `self.MovementComponent` (`SQHelicopter2.MovementComponent` _asbp_generic_helicopter))
  (set `self.ParentHeli` _asbp_generic_helicopter)
  (`KismetSystemLibrary.K2_SetTimerDelegate` (delegate `CollisionPrediction`) (`self.CollisionCheckInterval`) true))

(event `CollisionPrediction`
  (`self.DoCollisionWarning`))

(fn `DoCollisionWarning`
  (bind _parentheli (`self.ParentHeli`)
    (:`then`
      (if (`SQHelicopterInstruments.IsEngineActive` _parentheli)
        (bind _returnvalue (`Actor.GetVelocity` _parentheli))
        (bind _array (`|MakeArray` _parentheli :!type "Actor Object Reference"))
        (bind _willcollide (`self.StaticCompCollisionPrediction` (`SQHelicopter2.MainBladesCollision` _parentheli) _returnvalue _array))
        (bind _willcollide_2 (`self.StaticCompCollisionPrediction` (`SQHelicopter2.TailBladesCollision` _parentheli) _returnvalue _array))
        (bind _returnvalue_2 (or _willcollide_2 _willcollide))
        ;[1 1 1] Warning on heli (Network should be optimized)
        (if (!= _returnvalue_2 (`/Game/Vehicles/UH60M/BP_Generic_Helicopter.Warning On` _parentheli))
          (set `/Game/Vehicles/UH60M/BP_Generic_Helicopter.Warning On` _returnvalue_2 _parentheli))))
    (:`else`)))

(fn `DoHovering`
  (params (DeltaTime :type "Float (double-precision)"))
  (bind _movementcomponent (`self.MovementComponent`))
  (bind _maxflyspeed (`SQHelicopterMovementComponent.MaxFlySpeed` _movementcomponent))
  (bind _updatedcomponent (`SQHelicopterMovementComponent.UpdatedComponent` _movementcomponent))
  (bind _returnvalue (`KismetMathLibrary.NormalizedDeltaRotator` (`SQHelicopterMovementComponent.GetRotationInput` _movementcomponent) (`KismetMathLibrary.RInterpTo` (struct) (`KismetMathLibrary.MakeRotator` (+ (.roll (`SceneComponent.K2_GetComponentRotation` _updatedcomponent)) (`KismetMathLibrary.FMin` (* (/ (.y (`KismetMathLibrary.GreaterGreater_VectorRotator` (`SceneComponent.GetComponentVelocity` _updatedcomponent) (`KismetMathLibrary.MakeRotator` 0.0 0.0 (- 0.0 (.yaw (`SceneComponent.K2_GetComponentRotation` _updatedcomponent)))))) _maxflyspeed) (`self.VelocityRollCoef`)) (`self.MaxRollAngle`))) (- (`KismetMathLibrary.FMin` (* (/ (.x (`KismetMathLibrary.GreaterGreater_VectorRotator` (`SceneComponent.GetComponentVelocity` _updatedcomponent) (`KismetMathLibrary.MakeRotator` 0.0 0.0 (- 0.0 (.yaw (`SceneComponent.K2_GetComponentRotation` _updatedcomponent)))))) _maxflyspeed) (`self.VelocityPitchCoef`)) (`self.MaxPitchAngle`)) (.pitch (`SceneComponent.K2_GetComponentRotation` _updatedcomponent)))) DeltaTime (`self.InterpSpeed`))))
  (`/Engine/EditorBlueprintResources/StandardMacros.Can Execute Cosmetic Events`
    (:`True`
      (if (`self.EnableHovering`)
        (`SQHelicopterMovementComponent.AddRotationInput` _movementcomponent _returnvalue)
        (`KismetSystemLibrary.PrintString` (`KismetStringLibrary.Conv_RotatorToString` _returnvalue))))))

(fn `SetEnableHovering`
  (params (EnableHovering :type Boolean))
  (set `self.EnableHovering` EnableHovering))

(fn `StaticCompCollisionPrediction`
  (params (StaticComp :type "StaticMeshComponent Object Reference") (Velocity :type "Vector Structure") (ActorsToIgnore :type "Array of Actor Object Reference (by ref)"))
  (returns (WillCollide :type Boolean) (OutHit :type "HitResult Structure"))
  (bind (_min _max) (`StaticMeshComponent.GetLocalBounds` StaticComp))
  (bind _returnvalue (`SceneComponent.K2_GetComponentLocation` StaticComp))
  (bind (_outhit _returnvalue_2) (`KismetSystemLibrary.BoxTraceSingle` _returnvalue (+ _returnvalue (* Velocity (`self.CollisionPredictionTime`))) (/ (- _max _min) 2.0) (`SceneComponent.K2_GetComponentRotation` StaticComp) "TraceTypeQuery1" false ActorsToIgnore "ForDuration"))
  (return _returnvalue_2 _outhit))